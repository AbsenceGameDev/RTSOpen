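; BP_SpeakerPawn is a test pawn that starts and drives a CommonConversation dialogue as the Speaker, with a Listener as target.
; On BeginPlay it adds a participant component, loads the conversation database through an async game-feature action, then starts the entry conversation.
; When the instance waits for choices, it prints the last message and its options on screen.
; Valid key presses select an option and request the conversation to advance.
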(event Custom|BeginWaitingForChoices
  ;[1 1 1] Print Text for questions
  (bind _returnvalue (Class|PDConversationBPFL|GetPreviousMessage (Variables|Default|GetConvoPartComp)))
  (Class|PDConversationBPFL|PrintConversationMessagetoScreen self (.Message (Utilities|Struct|BreakClientConversationMessagePayload _returnvalue)) "(R=0.383843,G=0.833333,B=0.368924,A=1.000000)")
  (for _array_element (.Options (Utilities|Struct|BreakClientConversationMessagePayload _returnvalue))
    (Class|PDConversationBPFL|PrintConversationTexttoScreen self (Utilities|String|StringToName (Utilities|Select :Index (.ChoiceType (Utilities|Struct|BreakClientConversationOptionEntry _array_element)) :ServerOnly "" :UserChoiceAvailable "" :UserChoiceUnavailable "( Can't select )")) (.ChoiceText (Utilities|Struct|BreakClientConversationOptionEntry _array_element)) "(R=1.000000,G=0.415181,B=0.455003,A=1.000000)")))

(event EventBeginPlay
  (bind _returnvalue (Game|AddComponentbyClass "/Script/CommonConversationRuntime.ConversationParticipantComponent"))
  (Variables|Default|SetConvoPartComp _returnvalue)
  ;[1 1 1] Async action instance to load and activate the Conversation Database via our game-feature module
  (|ActionInstance "ConversationData"
    (:Succeeded
      (bind _returnvalue_2 (Class|ConversationLibrary|StartConversation "(TagName=\"Conversation.Entry.00\")" self "(TagName=\"Conversation.Participant.Speaker\")" (Variables|Default|GetListener) "(TagName=\"Conversation.Participant.Listener\")" "/Script/PDConversationHelper.PDConversationInstance"))
      (bind _aspdconversation_instance (Utilities|Casting|CastToPDConversationInstance _returnvalue_2))
      (bind _output_get (Variables|Default|SetBaseConversationInstance _aspdconversation_instance))
      (EventDispatchers|BindEventtoOnBeginWaitingforChoices _output_get (delegate Custom|BeginWaitingForChoices))
      (if (Variables|/Script/PDConversationHelper.PDConversationInstance|GetbWaitingForChoices _output_get)
        (CallFunction|BeginWaitingforChoices)))))

(event Input|KeyboardEvents|AnyKey
  (params (Key :type Key%20Structure :default "None"))
  ;[1 1 1] Simple testing
  (:Pressed
    (bind _returnvalue (Class|PDConversationBPFL|ProcessInputKey Key (Variables|Default|GetValid%20Keys))
      (:KEY_SUCCESS
        (Variables|Default|SetChoice _returnvalue)
        (bind _returnvalue_2 (Class|PDConversationBPFL|GetPreviousMessage (Variables|Default|GetConvoPartComp)))
        (Class|PDConversationBPFL|RequesttoAdvance (Variables|Default|GetBaseConversationInstance) (Variables|Default|GetConvoPartComp) (Utilities|Struct|MakeAdvanceConversationRequest (.ChoiceReference (Utilities|Struct|BreakClientConversationOptionEntry (Utilities|Array|Get(acopy) (.Options (Utilities|Struct|BreakClientConversationMessagePayload _returnvalue_2)) (Variables|Default|GetChoice)))) (.ExtraData (Utilities|Struct|BreakClientConversationOptionEntry (Utilities|Array|Get(acopy) (.Options (Utilities|Struct|BreakClientConversationMessagePayload _returnvalue_2)) (Variables|Default|GetChoice))))))
        (Development|PrintString (Utilities|String|Append "Selected{" (Utilities|String|ToString(Integer) (Variables|Default|GetChoice)) "}") true true "(R=0.000000,G=0.660000,B=1.000000,A=1.000000)" 1e+02)))))

(fn ConstructionScript)