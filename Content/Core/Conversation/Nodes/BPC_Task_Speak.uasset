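; BPC_Task_Speak is a conversation task node that shows one line of dialogue from a participant on screen.
; It finds the actor for its ParticipantTag and casts it to RTSOInteractableConversationActor for the speaker name, falling back to "Speaker" if that fails.
; It prints its Message in a fixed pink colour, then immediately returns an advance-conversation result.
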(fn ExecuteTaskNode
  (params (Context :type Conversation%20Context%20Structure%20%28by%20ref%29))
  (bind _returnvalue (Class|ConversationContextHelpers|GetConversationParticipantActor Context (Variables|Default|GetParticipant%20Tag)))
  (Class|PDConversationBPFL|PrintConversationTexttoScreen (.AsRTSOInteractable%20Conversation%20Actor (Utilities|Casting|CastToRTSOInteractableConversationActor _returnvalue)) (select (.bSuccess (Utilities|Casting|CastToRTSOInteractableConversationActor _returnvalue)) (Variables|/Script/RTSOpen.RTSOInteractableConversationActor|GetActorName (.AsRTSOInteractable%20Conversation%20Actor (Utilities|Casting|CastToRTSOInteractableConversationActor _returnvalue))) "Speaker") (Variables|Default|GetMessage) "(R=1.000000,G=0.503812,B=0.925278,A=1.000000)")
  (bind _returnvalue_2 (Class|ConversationContextHelpers|AdvanceConversation Context))
  (return _returnvalue_2))