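; BP_RTSOController is the RTS player controller that sets up the player's UI and relays marquee selection to it.
; BeginPlay creates an entity debug view and a minimap widget, stores both references and adds them to the viewport.
; The marquee selection override calls the parent, then passes the selection group and selected entities to the debug view if valid.
; An interact HUD creation branch is present but never runs.
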(event EventBeginPlay
  (Utilities|FlowControl|Sequence
    (:then_0
      (bind _returnvalue (UserInterface|CreateWidget "/Game/Core/AI/UI/WBP_EntityDebugView.WBP_EntityDebugView_C" self))
      (bind _output_get (Variables|Default|SetEntityDebugVIew _returnvalue))
      (UserInterface|Viewport|AddtoViewport _output_get 0))
    (:then_1
      (bind _returnvalue_2 (UserInterface|CreateWidget "/Game/Core/Widgets/MiniMap/WBP_RTSOMiniMap.WBP_RTSOMiniMap_C" self))
      (bind _output_get_2 (Variables|Default|SetMiniMapView _returnvalue_2))
      (UserInterface|Viewport|AddtoViewport _output_get_2 0))))

(fn ConstructionScript)

(fn OnMarqueeSelectionUpdated
  (params (SelectionGroup :type Integer) (NewSelection :type Array%20of%20Integers))
  (bind _entitydebugview (Variables|Default|GetEntityDebugVIew))
  (|CallParentFunction SelectionGroup NewSelection)
  (Utilities|IsValid _entitydebugview
    (:Is%20Valid
      (Default|NewSelectedEntities _entitydebugview SelectionGroup NewSelection)
      (return))
    (:Is%20Not%20Valid
      (return))))